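; BP_monitor is a moving detector that triggers a fail message when the player character enters its SphereCollider.
; The overlap sends OnShowFailUIMessage to all actors implementing BP_UI_interface.
; On BeginPlay it caches the world locations of Pos1 and Pos2 as start and end points.
; Tick moves it toward the end point at Speed, scaled by delta time, and snaps it back to the start on arrival, looping one way.
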(event `self.SphereCollider.OnComponentBeginOverlap`
  (params (OverlappedComponent :type "PrimitiveComponent Object Reference") (OtherActor :type "Actor Object Reference") (OtherComp :type "PrimitiveComponent Object Reference") (OtherBodyIndex :type Integer) (bFromSweep :type Boolean) (SweepResult :type "HitResult Structure (by ref)"))
  (if (== OtherActor (`GameplayStatics.GetPlayerCharacter` 0))
    (bind _outactors (`GameplayStatics.GetAllActorsWithInterface` "/Game/UI/BP_UI_interface.BP_UI_interface_C"))
    (message `/Game/UI/BP_UI_interface.OnShowFailUI` _outactors)))

(event `self.ReceiveBeginPlay`
  (set `self.beginPos` (`SceneComponent.K2_GetComponentLocation` (`self.pos1`)))
  (set `self.currentPos` (`self.beginPos`))
  (set `self.endPos` (`SceneComponent.K2_GetComponentLocation` (`self.pos2`))))

(event `self.ReceiveTick`
  (params (DeltaSeconds :type "Float (single-precision)"))
  (bind _output_get (set `self.TipTime` DeltaSeconds))
  (bind _output_get_2 (set `self.currentPos` (+ (`self.currentPos`) (* (`KismetMathLibrary.Normal` (- (`self.endPos`) (`self.currentPos`))) (* _output_get (`self.Speed`))))))
  (`self.K2_SetActorLocation` _output_get_2)
  (if (<= (`KismetMathLibrary.Vector_Distance` (`self.currentPos`) (`self.endPos`)) 2.0)
    (bind _output_get_3 (set `self.currentPos` (`self.beginPos`)))
    (`self.K2_SetActorLocation` _output_get_3)))

(fn `UserConstructionScript`)