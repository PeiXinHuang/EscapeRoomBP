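; Door actor that swings open when the player overlaps its box collider while holding both the key and the file.
; Custom events set the key and file flags.
; A timeline then drives the actor's yaw from a DoorAngle track, with no closing logic.
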(event `self.BoxCollider.OnComponentBeginOverlap`
  (params (OverlappedComponent :type "PrimitiveComponent Object Reference") (OtherActor :type "Actor Object Reference") (OtherComp :type "PrimitiveComponent Object Reference") (OtherBodyIndex :type Integer) (bFromSweep :type Boolean) (SweepResult :type "HitResult Structure (by ref)"))
  (if (== OtherActor (`GameplayStatics.GetPlayerCharacter` 0))
    (if (`self.hasGetKey`)
      (if (`self.hasGetFile`)
        (bind (_direction _doorangle) (`Timeline|Timeline`)
          (:`Update`
            (`self.K2_SetActorRotation` (`KismetMathLibrary.MakeRotator` 0.0 0.0 _doorangle))))))))

(event `/Game/BP/BP_Key_Interface.OnGetKeyEvent`
  (set `self.hasGetKey` true))

(event `/Game/BP/BP_File_Interface.OnGetFileEvent`
  (set `self.hasGetFile` true))

(fn `UserConstructionScript`)